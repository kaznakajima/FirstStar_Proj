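; BP_ArmBase is a base Blueprint for a usable arm, exposing start, tick and end calls that take a Player.
; An IsUsing flag gates these calls and forwards them to Exec hooks without passing the Player, with GetIsUsing exposing the state.
; Start and tick hooks are empty, apparently for child overrides.
; EndUseExec contains a guarded self-call that is skipped when reached through EndUse, which clears the flag first.
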(fn `EndUse`
  (params (Player :type "/Game/Matsumoto/BP_Player Object Reference"))
  (if (`self.isUsing`)
    (set `self.isUsing` false)
    (`self.EndUseExec`)))

(fn `EndUseExec`
  (if (`self.isUsing`)
    (`self.EndUseExec`)
    (set `self.isUsing` false)))

(fn `GetIsUsing`
  (returns (IsUsing :type Boolean))
  (return (`self.isUsing`)))

(fn `StartUse`
  (params (Player :type "/Game/Matsumoto/BP_Player Object Reference"))
  (if (not (`self.isUsing`))
    (set `self.isUsing` true)
    (`self.StartUseExec`)))

(fn `StartUseExec`)

(fn `UsingTick`
  (params (Player :type "/Game/Matsumoto/BP_Player Object Reference"))
  (if (`self.isUsing`)
    (`self.UsingTickExec`)))

(fn `UsingTickExec`)