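; Base Blueprint for player movement modes, exposing lifecycle, axis input and tick events that each receive the Player.
; On Enabled it applies its camera settings (length, offsets and transform) to the Player's spring arm; the other events are empty.
; CalcFlyHeight line-traces straight down from the Player on the Visibility channel, with one-frame debug drawing, and returns whether it hit and the distance.
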(event `Generated`
  (params (Player :type "/Game/Matsumoto/Player/BP_Player Object Reference")))

(event `Disabled`
  (params (Player :type "/Game/Matsumoto/Player/BP_Player Object Reference")))

(event `Enabled`
  (params (Player :type "/Game/Matsumoto/Player/BP_Player Object Reference"))
  (bind _springarm (`/Game/Matsumoto/Player/BP_Player.SpringArm` Player))
  (`|ExecutionSequence`
    (:`then_0`
      (set `SpringArmComponent.TargetArmLength` (`self.CameraLength`) _springarm)
      (set `SpringArmComponent.SocketOffset` (`self.SocketOffset`) _springarm)
      (set `SpringArmComponent.TargetOffset` (`self.TargetOffset`) _springarm)
      (`SceneComponent.K2_SetRelativeTransform` _springarm (`self.ArmTransform`) false false))))

(event `AxisMoveForward`
  (params (Player :type "/Game/Matsumoto/Player/BP_Player Object Reference") (AxisValue :type "Float (double-precision)")))

(event `AxisMoveRight`
  (params (Player :type "/Game/Matsumoto/Player/BP_Player Object Reference") (AxisValue :type "Float (double-precision)")))

(event `Tick`
  (params (Player :type "/Game/Matsumoto/Player/BP_Player Object Reference") (DeltaTime :type "Float (double-precision)")))

(fn `CalcFlyHeight`
  (params (Player :type "/Game/Matsumoto/Player/BP_Player Object Reference") (RayDistance :type "Float (double-precision)"))
  (returns (IsHit :type Boolean) (Distance :type "Float (double-precision)"))
  (bind _returnvalue (`Actor.K2_GetActorLocation` Player))
  (bind (_outhit _returnvalue_2) (`/Game/Matsumoto/Player/BP_Player.LineTraceByChannel` Player _returnvalue (+ _returnvalue (* (0.0 0.0 -1.0) RayDistance)) "TraceTypeQuery1" false "ForOneFrame" true (struct :`R` 1.0 :`A` 1.0) (struct :`G` 1.0 :`A` 1.0) 5.0))
  (return _returnvalue_2 (`.Distance` (`GameplayStatics.BreakHitResult` _outhit))))