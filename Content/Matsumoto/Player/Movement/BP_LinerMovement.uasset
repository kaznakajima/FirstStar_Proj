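; Player movement mode that confines the player to a vertical plane along its forward axis, like a side-scroller.
; Right input moves along that axis and sets facing, which Tick blends into a mesh turn; forward input moves vertically while flying.
; Tick freezes velocity and gravity during attacks.
; When flying, a height check stops climbing above the player's maximum or without ground detected, pushing the player down.
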(event `self.Enabled`
  (params (Player :type "/Game/Matsumoto/Player/BP_Player Object Reference"))
  (bind _charactermovement (`Character.CharacterMovement` Player))
  (`parent.Enabled` Player)
  (`MovementComponent.SetPlaneConstraintEnabled` _charactermovement true)
  (`MovementComponent.SetPlaneConstraintNormal` _charactermovement (`KismetMathLibrary.GreaterGreater_VectorRotator` (`Actor.GetActorForwardVector` Player) (struct :`Yaw` 90.0))))

(event `self.Tick`
  (params (Player :type "/Game/Matsumoto/Player/BP_Player Object Reference") (DeltaTime :type "Float (single-precision)"))
  (bind _returnvalue (`Actor.GetActorUpVector` Player))
  (bind _charactermovement (`Character.CharacterMovement` Player))
  (bind _charactermovement_2 (`Character.CharacterMovement` Player))
  (bind _velocity (`MovementComponent.Velocity` _charactermovement_2))
  (`|ExecutionSequence`
    (:`then_0`
      ;[1 1 1] 攻撃時に重力無効
      (if (`/Game/Matsumoto/Player/BP_Player.IsAttack` Player)
        (set `MovementComponent.Velocity` (0.0 0.0 0.0) _charactermovement)
        (set `CharacterMovementComponent.GravityScale` 0.0 _charactermovement)
        (else
          (set `CharacterMovementComponent.GravityScale` 1.0 _charactermovement)
          (if (`NavMovementComponent.IsFlying` _charactermovement)
            (bind (_ishit _distance) (`self.CalcFlyHeight` Player 300.0))
            (if (or (not _ishit) (> _distance (`/Game/Matsumoto/Player/BP_Player.MaxFlyHeight` Player)))
              (if (< (`KismetMathLibrary.DegAcos` (`KismetMathLibrary.Dot_VectorVector` (`KismetMathLibrary.Normal` _velocity) (`KismetMathLibrary.Normal` _returnvalue))) 90.0)
                (set `MovementComponent.Velocity` (`KismetMathLibrary.ProjectVectorOnToPlane` _velocity _returnvalue) _charactermovement_2)
                (else
                  (set `MovementComponent.Velocity` (+ _velocity (* (* _returnvalue -1.0) (`self.FallSpeed`))) _charactermovement_2)))
              (`Pawn.AddMovementInput` Player _returnvalue (`KismetMathLibrary.FMin` (* (`self.VerticalMoveValue`) -1.0)) true))))))
    (:`then_1`
      ;[1 1 1] Player Rotation Tick
      (bind _output_get (set `self.RightRotationRatio` (`KismetMathLibrary.FClamp` (+ (* DeltaTime (`self.RotateSpeed`) (`KismetMathLibrary.SelectFloat` -1.0 1.0 (`self.IsRight`))) (`self.RightRotationRatio`)))))
      (`SceneComponent.K2_SetRelativeRotation` (`Character.Mesh` Player) (`KismetMathLibrary.RLerp` (struct) (struct :`Yaw` -180.0) _output_get true) false false))))

(event `self.AxisMoveRight`
  (params (Player :type "/Game/Matsumoto/Player/BP_Player Object Reference") (AxisValue :type "Float (single-precision)"))
  (`Pawn.AddMovementInput` Player (`Actor.GetActorForwardVector` Player) AxisValue false)
  (`Pawn.AddMovementInput` Player (`Actor.GetActorForwardVector` Player) AxisValue false)
  (if (!= AxisValue 0.0)
    (set `self.IsRight` (> AxisValue 0.0))))

(event `self.AxisMoveForward`
  (params (Player :type "/Game/Matsumoto/Player/BP_Player Object Reference") (AxisValue :type "Float (single-precision)"))
  (set `self.VerticalMoveValue` AxisValue)
  (if (`NavMovementComponent.IsFlying` (`Character.CharacterMovement` Player))
    (`Pawn.AddMovementInput` Player (`Actor.GetActorUpVector` Player) AxisValue false)))