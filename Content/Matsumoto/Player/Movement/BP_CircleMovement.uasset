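; Player movement component that confines the player to a circular path around a center point, facing along the tangent.
; On enable it lifts the plane constraint and records the radius, then re-projects location and rotation onto the circle each tick.
; Right-axis input moves along the forward vector.
; Tick also freezes velocity and gravity during attacks, and drives flying ascent or descent from the jump key, using a ground trace to cap height.
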(event `self.Enabled`
  (params (Player :type "/Game/Matsumoto/Player/BP_Player Object Reference"))
  (`parent.Enabled` Player)
  (`MovementComponent.SetPlaneConstraintEnabled` (`Character.CharacterMovement` Player) false)
  (bind _vector (`self.GetCircleVector` Player))
  (set `self.Radius` (`KismetMathLibrary.VSize` _vector)))

(event `self.Tick`
  (params (Player :type "/Game/Matsumoto/Player/BP_Player Object Reference") (DeltaTime :type "Float (single-precision)"))
  (bind _returnvalue (`Actor.K2_GetActorLocation` Player))
  (bind _charactermovement (`Character.CharacterMovement` Player))
  (bind _returnvalue_2 (* (`.JumpPower_11_26F02FCB457AE11E010B649498415B53` (break `/Game/Matsumoto/Player/S_PlayerStatusSet` (`/Game/Matsumoto/Player/BP_Player.PlayerParameter` Player))) DeltaTime))
  (`|ExecutionSequence`
    (:`then_0`
      (if (`/Game/Matsumoto/Player/BP_Player.IsAttack` Player)
        (set `MovementComponent.Velocity` (0.0 0.0 0.0) _charactermovement)
        (set `CharacterMovementComponent.GravityScale` 0.0 _charactermovement)
        (else
          (set `CharacterMovementComponent.GravityScale` 1.0 _charactermovement)
          (if (`NavMovementComponent.IsFlying` _charactermovement)
            (if (`/Game/Matsumoto/Player/BP_Player.IsPressJumpKey` Player)
              (bind (_outhit _returnvalue_3) (`/Game/Matsumoto/Player/BP_Player.LineTraceByChannel` Player _returnvalue (+ _returnvalue (* (0.0 0.0 -1.0) 300.0)) "TraceTypeQuery1" false "ForOneFrame" true (struct :`R` 1.0 :`A` 1.0) (struct :`G` 1.0 :`A` 1.0) 5.0))
              (if _returnvalue_3
                (if (not (> (+ (`.Distance` (`GameplayStatics.BreakHitResult` _outhit)) _returnvalue_2) (`/Game/Matsumoto/Player/BP_Player.MaxFlyHeight` Player)))
                  ;[1 1 1] Fly
                  (`Actor.K2_AddActorWorldOffset` Player (`KismetMathLibrary.MakeVector` 0.0 0.0 _returnvalue_2) true false))
                (else
                  ;[1 1 1] Fall
                  (`Actor.K2_AddActorWorldOffset` Player (`KismetMathLibrary.MakeVector` 0.0 0.0 (* -1.0 _returnvalue_2)) true false :!label _label)))
              (else
                (goto _label)))))))
    (:`then_1`
      ;[1 1 1] Constraint
      (bind _rotation (`self.GetRotation` Player))
      (bind _vector (`self.GetCircleVector` Player))
      (`Actor.K2_SetActorLocationAndRotation` Player (+ (* (`KismetMathLibrary.Normal` _vector) (`self.Radius`)) (`KismetMathLibrary.MakeVector` 0.0 0.0 (.z (`Actor.K2_GetActorLocation` Player)))) _rotation false false))))

(event `self.AxisMoveRight`
  (params (Player :type "/Game/Matsumoto/Player/BP_Player Object Reference") (AxisValue :type "Float (single-precision)"))
  (`Pawn.AddMovementInput` Player (`Actor.GetActorForwardVector` Player) AxisValue false))

(fn `GetCircleVector`
  (params (Player :type "/Game/Matsumoto/Player/BP_Player Object Reference"))
  (returns (Vector :type "Vector Structure"))
  (return (`KismetMathLibrary.MakeVector` (.x (- (`Actor.K2_GetActorLocation` Player) (`self.CenterPositionXY`))) (.y (- (`Actor.K2_GetActorLocation` Player) (`self.CenterPositionXY`))))))

(fn `GetRotation`
  (params (Player :type "/Game/Matsumoto/Player/BP_Player Object Reference"))
  (returns (Rotation :type "Rotator Structure"))
  (bind _vector (`self.GetCircleVector` Player))
  (return (`KismetMathLibrary.MakeRotFromX` (`KismetMathLibrary.GreaterGreater_VectorRotator` _vector (struct :`Yaw` -90.0)))))