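; Player body Blueprint that animates idle, damage, death and attacks (taps, stretch, rolling tap, predation) through a component-based state machine.
; Construction registers state components, disables sphere and box colliders, and creates dynamic materials for body meshes.
; Each handled state plays a timeline that transforms body parts, with event tracks toggling attack hitboxes; most states chain back to Idle.
; Dynamic material parameters drive the damage flash and star-power ratio.
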(event `self.StateDamage.OnBeginState`
  (bind _playermaterialdynamic (`self.PlayerMaterialDynamic`))
  (bind _parent (`self.Parent`))
  ;[1 1 1] Damage Animation
  (`|ExecutionSequence`
    (:`then_0`
      (bind (_direction _position _rotation) (`Timeline|Damage` :!via `PlayFromStart` :!label _label)
        (:`Update`
          (`SceneComponent.K2_SetRelativeLocation` _parent _position false false)
          (`SceneComponent.K2_SetRelativeRotation` _parent (`KismetMathLibrary.MakeRotator` (.x _rotation) (.y _rotation) (.z _rotation)) false false))))
    (:`then_1`
      (for _array_element _playermaterialdynamic
        (`MaterialInstanceDynamic.SetScalarParameterValue` _array_element "IsDamage" 1.0)
        (`KismetSystemLibrary.Delay` 0.2)
        (for _array_element_2 _playermaterialdynamic
          (`MaterialInstanceDynamic.SetScalarParameterValue` _array_element_2 "IsDamage" 0.0))))))

(event `self.StateDamage.OnEndState`
  (bind _parent (`self.Parent`))
  ;[1 1 1] Damage Animation
  (`|ExecutionSequence`
    (:`then_0`
      (goto _label :!via `Stop`))
    (:`then_1`
      (`SceneComponent.K2_SetRelativeLocation` _parent (0.0 0.0 0.0) false false)
      (`SceneComponent.K2_SetRelativeRotation` :`self` _parent))))

(event `self.ReceiveBeginPlay`
  (`|ExecutionSequence`
    (:`then_0`
      ;[1 1 1] Set Next State
      (`|ExecutionSequence`
        (:`then_0`
          (`/Game/Matsumoto/StateMachine/StateBaseComponent.SetNextState` (`self.StateDamage`) (`self.StateIdle`)))
        (:`then_1`
          (`/Game/Matsumoto/StateMachine/StateBaseComponent.SetNextState` (`self.StateLeftTap`) (`self.StateIdle`)))
        (:`then_2`
          (`/Game/Matsumoto/StateMachine/StateBaseComponent.SetNextState` (`self.StateRightTap`) (`self.StateIdle`)))
        (:`then_3`
          (`/Game/Matsumoto/StateMachine/StateBaseComponent.SetNextState` (`self.StateRollingTap`) (`self.StateIdle`)))
        (:`then_4`
          (`/Game/Matsumoto/StateMachine/StateBaseComponent.SetNextState` (`self.StatePredation`) (`self.StateIdle`)))
        (:`then_5`
          (`/Game/Matsumoto/StateMachine/StateBaseComponent.SetNextState` (`self.StateRightStretch`) (`self.StateIdle`)))
        (:`then_6`
          (`/Game/Matsumoto/StateMachine/StateBaseComponent.SetNextState` (`self.StateLeftStretch`) (`self.StateIdle`)))))
    (:`then_1`
      ;[1 1 1] Run State
      (`/Game/Matsumoto/StateMachine/StateMachineComponent.Start` (`self.StateMachineComponent`) "StateIdle"))))

(event `self.StateIdle.OnBeginState`
  ;[1 1 1] Idle Animation
  (bind (_direction _position) (`Timeline|Idle` :!via `PlayFromStart` :!label _label_2)
    (:`Update`
      (`SceneComponent.K2_SetRelativeLocation` (`self.Parent`) _position false false))))

(event `self.StateIdle.OnEndState`
  ;[1 1 1] Idle Animation
  (`|ExecutionSequence`
    (:`then_0`
      (goto _label_2 :!via `Stop`))
    (:`then_1`
      (`SceneComponent.K2_SetRelativeLocation` (`self.Parent`) (0.0 0.0 0.0) false false))))

(event `self.StateLeftTap.OnBeginState`
  (bind _lefttapcol (`self.LeftTapCol`))
  ;[1 1 1] LeftTap Animation
  (bind (_direction _rotation _scale) (`Timeline|TapLeft` :!via `PlayFromStart` :!label _label_3)
    (:`Update`
      (`SceneComponent.SetRelativeScale3D` (`self.LeftArm`) _scale)
      (`SceneComponent.K2_SetRelativeRotation` (`self.LeftArmCenter`) (`KismetMathLibrary.MakeRotator` (.x _rotation) (.y _rotation) (.z _rotation)) false false))
    (:`CollisionEnable`
      (`self.SetCollision` _lefttapcol true))
    (:`CollisionDisable`
      (`self.SetCollision` _lefttapcol))))

(event `self.StateDeath.OnBeginState`
  (bind _parent (`self.Parent`))
  ;[1 1 1] Death Animation
  (bind (_direction _position _rotation) (`Timeline|Death` :!via `PlayFromStart`)
    (:`Update`
      (`SceneComponent.K2_SetRelativeLocation` _parent _position false false)
      (`SceneComponent.K2_SetRelativeRotation` _parent (`KismetMathLibrary.MakeRotator` (.x _rotation) (.y _rotation) (.z _rotation)) false false))))

(event `self.StateLeftStretch.OnBeginState`
  (bind _leftstretchcol (`self.LeftStretchCol`))
  (bind (_direction _rotation _scale) (`Timeline|StretchLeft` :!via `PlayFromStart` :!label _label_4)
    (:`Update`
      (`SceneComponent.SetRelativeScale3D` (`self.LeftArm`) _scale)
      (`SceneComponent.K2_SetRelativeRotation` (`self.LeftArmRot`) (`KismetMathLibrary.MakeRotator` (.x _rotation) (.y _rotation) (.z _rotation)) false false))
    (:`CollisionEnable`
      (`self.SetCollision` _leftstretchcol true))
    (:`CollisionDisable`
      (`self.SetCollision` _leftstretchcol))))

(event `self.StateLeftTap.OnEndState`
  ;[1 1 1] LeftTap Animation
  (`|ExecutionSequence`
    (:`then_0`
      (goto _label_3 :!via `Stop`))
    (:`then_1`
      (`SceneComponent.SetRelativeScale3D` (`self.LeftArm`) (0.4 0.4 0.4))
      (`SceneComponent.K2_SetRelativeRotation` :`self` (`self.LeftArmCenter`)))))

(event `self.StateLeftStretch.OnEndState`
  (`|ExecutionSequence`
    (:`then_0`
      (goto _label_4 :!via `Stop`))
    (:`then_1`
      (`SceneComponent.SetRelativeScale3D` (`self.LeftArm`) (0.4 0.4 0.4))
      (`SceneComponent.K2_SetRelativeRotation` (`self.LeftArmRot`) (struct :`Roll` 108.0) false false))))

(event `self.StatePredation.OnBeginState`
  (bind _predationcol (`self.PredationCol`))
  ;[1 1 1] Predation Animation
  (bind (_direction _rotation _transform) (`Timeline|Predation` :!via `PlayFromStart` :!label _label_5)
    (:`Update`
      (`|ExecutionSequence`
        (:`then_0`
          (`SceneComponent.K2_SetRelativeLocationAndRotation` (`self.Head`) _transform (`KismetMathLibrary.MakeRotator` (.x _rotation) (.y _rotation) (.z _rotation)) false false))
        (:`then_1`
          (`SceneComponent.K2_SetRelativeLocationAndRotation` (`self.RightArm`) _transform (`KismetMathLibrary.MakeRotator` (.x _rotation) (.y _rotation) (.z _rotation)) false false))
        (:`then_2`
          (`SceneComponent.K2_SetRelativeLocationAndRotation` (`self.LeftArm`) _transform (`KismetMathLibrary.MakeRotator` (.x _rotation) (.y _rotation) (.z _rotation)) false false))
        (:`then_3`
          (`SceneComponent.K2_SetRelativeLocationAndRotation` (`self.RightFoot`) _transform (`KismetMathLibrary.MakeRotator` (.x _rotation) (.y _rotation) (.z _rotation)) false false))
        (:`then_4`
          (`SceneComponent.K2_SetRelativeLocationAndRotation` (`self.LeftFoot`) _transform (`KismetMathLibrary.MakeRotator` (.x _rotation) (.y _rotation) (.z _rotation)) false false))))
    (:`CollisionEnable`
      (`self.SetCollision` _predationcol true))
    (:`CollisionDisable`
      (`self.SetCollision` _predationcol))))

(event `self.StatePredation.OnEndState`
  ;[1 1 1] Predation Animation
  (`|ExecutionSequence`
    (:`then_0`
      (goto _label_5 :!via `Stop`))
    (:`then_1`
      (`SceneComponent.K2_SetRelativeLocationAndRotation` :`self` (`self.Head`)))
    (:`then_2`
      (`SceneComponent.K2_SetRelativeLocationAndRotation` :`self` (`self.RightArm`)))
    (:`then_3`
      (`SceneComponent.K2_SetRelativeLocationAndRotation` :`self` (`self.LeftArm`)))
    (:`then_4`
      (`SceneComponent.K2_SetRelativeLocationAndRotation` :`self` (`self.RightFoot`)))
    (:`then_5`
      (`SceneComponent.K2_SetRelativeLocationAndRotation` :`self` (`self.LeftFoot`)))))

(event `self.StateRightTap.OnBeginState`
  (bind _righttapcol (`self.RightTapCol`))
  ;[1 1 1] Right Tap Animation
  (bind (_direction _rotation _scale) (`Timeline|TapRight` :!via `PlayFromStart` :!label _label_6)
    (:`Update`
      (`SceneComponent.SetRelativeScale3D` (`self.RightArm`) _scale)
      (`SceneComponent.K2_SetRelativeRotation` (`self.RightArmCenter`) (`KismetMathLibrary.MakeRotator` (.x _rotation) (.y _rotation) (.z _rotation)) false false))
    (:`CollisionEnable`
      (`self.SetCollision` _righttapcol true))
    (:`CollisionDisable`
      (`self.SetCollision` _righttapcol))))

(event `self.StateRightTap.OnEndState`
  ;[1 1 1] Right Tap Animation
  (`|ExecutionSequence`
    (:`then_0`
      (goto _label_6 :!via `Stop`))
    (:`then_1`
      (`SceneComponent.SetRelativeScale3D` (`self.RightArm`) (0.4 0.4 0.4))
      (`SceneComponent.K2_SetRelativeRotation` :`self` (`self.RightArmCenter`)))))

(event `self.StateRollingTap.OnBeginState`
  (bind _rollingtapcol (`self.RollingTapCol`))
  ;[1 1 1] Rolling Tap Animation
  (bind (_direction _rotation _scale) (`Timeline|TapRolling` :!via `PlayFromStart` :!label _label_7)
    (:`Update`
      (`SceneComponent.SetRelativeScale3D` (`self.RightArm`) _scale)
      (`SceneComponent.SetRelativeScale3D` (`self.LeftArm`) _scale)
      (`SceneComponent.K2_SetRelativeRotation` (`self.Parent`) (`KismetMathLibrary.MakeRotator` (.x _rotation) (.y _rotation) (.z _rotation)) false false))
    (:`CollisionEnable`
      (`self.SetCollision` _rollingtapcol true))
    (:`CollisionDisable`
      (`self.SetCollision` _rollingtapcol))))

(event `self.StateRollingTap.OnEndState`
  ;[1 1 1] Rolling Tap Animation
  (`|ExecutionSequence`
    (:`then_0`
      (goto _label_7 :!via `Stop`))
    (:`then_1`
      (`SceneComponent.SetRelativeScale3D` (`self.RightArm`) (0.4 0.4 0.4))
      (`SceneComponent.SetRelativeScale3D` (`self.LeftArm`) (0.4 0.4 0.4))
      (`SceneComponent.K2_SetRelativeRotation` :`self` (`self.Parent`)))))

(fn `SetCollision`
  (params (Component :type "PrimitiveComponent Object Reference") (Enabled :type Boolean))
  (if Enabled
    (`PrimitiveComponent.SetCollisionEnabled` Component "QueryAndPhysics")
    (else
      (`PrimitiveComponent.SetCollisionEnabled` Component "NoCollision"))))

(fn `SetStarPowerRatio`
  (params (StarPowerRatio :type "Float (double-precision)"))
  (for _array_element (`self.PlayerMaterialDynamic`)
    (`MaterialInstanceDynamic.SetScalarParameterValue` _array_element "StarRatio" StarPowerRatio)))

(fn `UserConstructionScript`
  (locals (Collisions :type "Array of PrimitiveComponent Object Reference"))
  (`|ExecutionSequence`
    (:`then_0`
      ;[1 1 1] Add ModelSet
      (for _array_element (`SceneComponent.GetChildrenComponents` (`self.BodyBase`) true)
        (`BlueprintMapLibrary.Map_Add` (`self.BodySet`) (`KismetSystemLibrary.GetObjectName` _array_element) _array_element))
      ;[1 1 1] Create & Apply Dynamic Material Instance
      (bind _values (`BlueprintMapLibrary.Map_Values` (`self.BodySet`)))
      (for _array_element_2 _values
        (bind _asstatic_mesh_component (cast `StaticMeshComponent` _array_element_2))
        (bind _returnvalue (`PrimitiveComponent.CreateDynamicMaterialInstance` _asstatic_mesh_component 0 (`PrimitiveComponent.GetMaterial` _asstatic_mesh_component 0) "None"))
        (`KismetArrayLibrary.Array_Add` (`self.PlayerMaterialDynamic`) _returnvalue)))
    (:`then_1`
      ;[1 1 1] Set Up Collision
      (`|ExecutionSequence`
        (:`then_0`
          (for _array_element_3 (`self.K2_GetComponentsByClass` "/Script/Engine.SphereComponent")
            (`self.SetCollision` _array_element_3)))
        (:`then_1`
          (for _array_element_4 (`self.K2_GetComponentsByClass` "/Script/Engine.BoxComponent")
            (`self.SetCollision` _array_element_4)))))
    (:`then_2`
      ;[1 1 1] Add State
      (for _array_element_5 (`self.K2_GetComponentsByClass` "/Game/Matsumoto/StateMachine/StateBaseComponent.StateBaseComponent_C")
        (`/Game/Matsumoto/StateMachine/StateMachineComponent.AddState` (`self.StateMachineComponent`) _array_element_5)))))