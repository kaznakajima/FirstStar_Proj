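; BP_Stretch is the player's "Stretch" arm weapon, a melee attack driven by the player's animation Blueprint.
; On generation it binds left and right stretch colliders and subscribes to AnimBP attack events, which switch each collider on and off.
; Using it triggers the AnimBP stretch attack, and hits apply base power as damage with a debug print.
; The start of either side's combo event ends the current use.
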(event `self.StartUseChild`
  (params (Player :type "/Game/Matsumoto/Player/BP_Player Object Reference"))
  (`/Game/Matsumoto/Player/StarModel/Star_AnimBP.StretchAttackEvent` (`/Game/Matsumoto/Player/BP_Player.AnimBP` Player)))

(event `self.UsingTickChild`
  (params (DeltaTime :type "Float (single-precision)") (Player :type "/Game/Matsumoto/Player/BP_Player Object Reference")))

(event `LeftStretchAttackEnd`
  ;[1 1 1] Bind Collision
  (`/Game/Matsumoto/Player/BP_Player.SetCollision` (stale `self.Generated` Player) (stale `self.Generated` _primitivecomponent) false))

(event `LeftStretchAttackStart`
  ;[1 1 1] Bind Collision
  (`/Game/Matsumoto/Player/BP_Player.SetCollision` (stale `self.Generated` Player) (stale `self.Generated` _primitivecomponent) true))

(event `self.EndUseChild`
  (params (Player :type "/Game/Matsumoto/Player/BP_Player Object Reference"))
  (`self.ShowMessage` "EndStretch"))

(event `self.Generated`
  (params (Player :type "/Game/Matsumoto/Player/BP_Player Object Reference"))
  (bind _animbp (`/Game/Matsumoto/Player/BP_Player.AnimBP` Player))
  (bind _animbp_2 (`/Game/Matsumoto/Player/BP_Player.AnimBP` Player))
  (bind _animbp_3 (`/Game/Matsumoto/Player/BP_Player.AnimBP` Player))
  (`|ExecutionSequence`
    (:`then_0`
      ;[1 1 1] Bind Collision
      (`|ExecutionSequence`
        (:`then_0`
          (bind _primitivecomponent (`self.BindCollisionEvent` Player "LeftStretchCol"))
          (add `/Game/Matsumoto/Player/StarModel/Star_AnimBP.OnLeftStretchAttackStarted` _animbp_2 (delegate `LeftStretchAttackStart`))
          (add `/Game/Matsumoto/Player/StarModel/Star_AnimBP.OnLeftStretchAttackEnded` _animbp_2 (delegate `LeftStretchAttackEnd`)))
        (:`then_1`
          (bind _primitivecomponent_2 (`self.BindCollisionEvent` Player "RightStretchCol"))
          (add `/Game/Matsumoto/Player/StarModel/Star_AnimBP.OnRightStretchAttackStarted` _animbp (delegate `RightStretchAttackStart`))
          (add `/Game/Matsumoto/Player/StarModel/Star_AnimBP.OnRightStretchAttackEnded` _animbp (delegate `RightStretchAttackEnd`)))))
    (:`then_1`
      ;[1 1 1] Bind Combo
      (add `/Game/Matsumoto/Player/StarModel/Star_AnimBP.OnLeftStretchComboStarted` _animbp_3 (delegate `OnComboStart`))
      (add `/Game/Matsumoto/Player/StarModel/Star_AnimBP.OnRightStretchComboStarted` _animbp_3 (delegate `OnComboStart`)))))

(event `RightStretchAttackEnd`
  ;[1 1 1] Bind Collision
  (`/Game/Matsumoto/Player/BP_Player.SetCollision` (stale `self.Generated` Player) (stale `self.Generated` _primitivecomponent_2) false))

(event `RightStretchAttackStart`
  ;[1 1 1] Bind Collision
  (`/Game/Matsumoto/Player/BP_Player.SetCollision` (stale `self.Generated` Player) (stale `self.Generated` _primitivecomponent_2) true))

(event `self.CollisionHitChild`
  (params (OverlappedComponent :type "PrimitiveComponent Object Reference") (OtherActor :type "Actor Object Reference") (OtherCompoent :type "PrimitiveComponent Object Reference") (OtherBodyIndex :type Integer) (FromSweep :type Boolean) (SweepResult :type "HitResult Structure"))
  (bind _basepower (`self.BasePower`))
  (`GameplayStatics.ApplyDamage` OtherActor _basepower)
  (`KismetSystemLibrary.PrintString` null (`KismetStringLibrary.Concat_StrStr` "Hit Damage : " (`KismetStringLibrary.Conv_DoubleToString` _basepower))))

(event `OnComboStart`
  (`self.EndUse` (stale `self.Generated` Player)))

(fn `GetWeaponName`
  (returns (WeaponName :type Text))
  (return "Stretch"))