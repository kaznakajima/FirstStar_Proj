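; Base Blueprint for the player's arm weapons, defining a shared use lifecycle of start, per-tick update and end.
; An IsUsing flag gates each stage, which calls an overridable child function and then fires an event dispatcher.
; BindCollisionEvent looks up player collision components by name and binds their begin-overlap, forwarding hits on anything except BP_Player.
; Ending use disables every bound collision through the player.
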(event `StartUse`
  (params (Player :type "/Game/Matsumoto/Player/BP_Player Object Reference"))
  ;[1 1 1] Start Use
  (if (not (`self.IsUsing`))
    (set `self.IsUsing` true)
    (`self.StartUseChild` Player)
    (`self.OnStartUse` Player)))

(event `EquipTick`
  (params (DeltaTime :type "Float (double-precision)") (Player :type "/Game/Matsumoto/Player/BP_Player Object Reference"))
  ;[1 1 1] Tick
  (if (`self.IsUsing`)
    (`self.UsingTickChild` DeltaTime Player)
    (`self.OnUseTick` DeltaTime Player)))

(event `EndUse`
  (params (Player :type "/Game/Matsumoto/Player/BP_Player Object Reference"))
  ;[1 1 1] End Use
  (if (`self.IsUsing`)
    (`|ExecutionSequence`
      (:`then_0`
        (for _array_element (`self.BindedCollisions`)
          (`/Game/Matsumoto/Player/BP_Player.SetCollision` Player _array_element false)))
      (:`then_1`
        (set `self.IsUsing` false)
        (`self.EndUseChild` Player)
        (`self.OnEndUse` Player)))))

(event `CollisionHit`
  (params (OverlappedComponent :type "PrimitiveComponent Object Reference") (OtherActor :type "Actor Object Reference") (OtherComponent :type "PrimitiveComponent Object Reference") (OtherBodyIndex :type Integer) (FromSweep :type Boolean) (SweepResult :type "HitResult Structure (by ref)"))
  (cast `/Game/Matsumoto/Player/BP_Player` OtherActor
    (:`CastFailed`
      (`self.CollisionHitChild` OverlappedComponent OtherActor OtherComponent OtherBodyIndex FromSweep SweepResult)
      (`self.OnCollisionHit` OverlappedComponent OtherActor OtherComponent OtherBodyIndex FromSweep SweepResult))))

(fn `BindCollisionEvent`
  (params (Player :type "/Game/Matsumoto/Player/BP_Player Object Reference") (ComponentName :type String))
  (returns (PrimitiveComponent :type "PrimitiveComponent Object Reference"))
  (bind (_value _returnvalue) (`BlueprintMapLibrary.Map_Find` (`/Game/Matsumoto/Player/BP_Player.Collisions` Player) ComponentName))
  (if _returnvalue
    (add `PrimitiveComponent.OnComponentBeginOverlap` _value (`|CreateDelegate` :!event `CollisionHit`))
    (add `PrimitiveComponent.OnComponentBeginOverlap` _value (`|CreateDelegate` :!event `CollisionHit`))
    (`KismetArrayLibrary.Array_Add` (`self.BindedCollisions`) _value)
    (return _value)
    (else
      (`KismetSystemLibrary.PrintString` null "Component is not found" true true (struct :`R` 1.0 :`G` 0.023868 :`A` 1.0)))))

(fn `CollisionHitChild`
  (params (OverlappedComponent :type "PrimitiveComponent Object Reference") (OtherActor :type "Actor Object Reference") (OtherCompoent :type "PrimitiveComponent Object Reference") (OtherBodyIndex :type Integer) (FromSweep :type Boolean) (SweepResult :type "HitResult Structure"))
  (return))

(fn `EndUseChild`
  (params (Player :type "/Game/Matsumoto/Player/BP_Player Object Reference")))

(fn `Generated`
  (params (Player :type "/Game/Matsumoto/Player/BP_Player Object Reference")))

(fn `GetIsUsing`
  (returns (IsUsing :type Boolean))
  (return (`self.IsUsing`)))

(fn `GetWeaponName`
  (returns (WeaponName :type Text))
  (return "Not Set"))

(fn `ShowMessage`
  (params (Message :type String :default "Hello"))
  (if (`self.DisplayDebugMessage`)
    (`KismetSystemLibrary.PrintString` null Message)))

(fn `StartUseChild`
  (params (Player :type "/Game/Matsumoto/Player/BP_Player Object Reference")))

(fn `UsingTickChild`
  (params (DeltaTime :type "Float (double-precision)") (Player :type "/Game/Matsumoto/Player/BP_Player Object Reference")))