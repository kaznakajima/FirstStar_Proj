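; Player arm equipment for a tap attack, damaging actors hit by its left, right and rolling colliders.
; On generation it binds the three collision events, and each hit deals base power scaled by the current TapState's multiplier.
; A timed three-step combo that drives player body animation states is present but disconnected, so use start does nothing and TapState never advances.
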(event `self.StartUseChild`
  (params (Player :type "/Game/Matsumoto/Player/BP_Player Object Reference")))

(event `self.EquipTick`
  (params (DeltaTime :type "Float (single-precision)") (Player :type "/Game/Matsumoto/Player/BP_Player Object Reference"))
  (`parent.EquipTick` DeltaTime Player)
  (bind _output_get (set `self.InputElapcedTime` (+ DeltaTime (`self.InputElapcedTime`)))))

(event `self.EndUseChild`
  (params (Player :type "/Game/Matsumoto/Player/BP_Player Object Reference"))
  (`self.ShowMessage` "EndTap"))

(event `self.OnGenerated`
  (params (Player :type "/Game/Matsumoto/Player/BP_Player Object Reference"))
  (`|ExecutionSequence`
    (:`then_0`
      ;[1 1 1] Bind Hit Event
      (`|ExecutionSequence`
        (:`then_0`
          (`self.BindCollisionEvent` Player "LeftTapCol"))
        (:`then_1`
          (`self.BindCollisionEvent` Player "RightTapCol"))
        (:`then_2`
          (`self.BindCollisionEvent` Player "RollingTapCol"))))))

(event `EndAnimation`
  ;[1 1 1] Bind Event
  ;[1 1 1] Combo Start
  (set `self.InputElapcedTime` 0.0))

(event `self.CollisionHitChild`
  (params (OverlappedComponent :type "PrimitiveComponent Object Reference") (OtherActor :type "Actor Object Reference") (OtherCompoent :type "PrimitiveComponent Object Reference") (OtherBodyIndex :type Integer) (FromSweep :type Boolean) (SweepResult :type "HitResult Structure"))
  (bind _returnvalue (* (`self.BasePower`) (`|GetArrayItem` (`self.DamageMList`) (`self.TapState`))))
  ;[1 1 1] On Hit
  (`GameplayStatics.ApplyDamage` OtherActor _returnvalue)
  (`KismetSystemLibrary.PrintString` null (`KismetStringLibrary.Concat_StrStr` "Hit Damage : " (`KismetStringLibrary.Conv_DoubleToString` _returnvalue))))