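; BP_PredationArm is a player arm weapon named "Predation" that performs an eating melee attack.
; Use triggers the predation attack on the player's AnimBP, whose callbacks toggle the PredationCol hit collision and end the use.
; Hits play an eat sound and apply base-power damage, also granting a fixed amount of StarPower when the target is an enemy character.
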(event `self.StartUseChild`
  (params (Player :type "/Game/Matsumoto/Player/BP_Player Object Reference"))
  (`/Game/Matsumoto/Player/StarModel/Star_AnimBP.PredationAttackEvent` (`/Game/Matsumoto/Player/BP_Player.AnimBP` Player)))

(event `self.UsingTickChild`
  (params (DeltaTime :type "Float (single-precision)") (Player :type "/Game/Matsumoto/Player/BP_Player Object Reference")))

(event `self.EndUseChild`
  (params (Player :type "/Game/Matsumoto/Player/BP_Player Object Reference")))

(event `self.Generated`
  (params (Player :type "/Game/Matsumoto/Player/BP_Player Object Reference"))
  (bind _animbp (`/Game/Matsumoto/Player/BP_Player.AnimBP` Player))
  (`parent.Generated` Player)
  (`|ExecutionSequence`
    (:`then_0`
      ;[1 1 1] Bind Collision
      (bind _primitivecomponent (`self.BindCollisionEvent` Player "PredationCol"))
      (add `/Game/Matsumoto/Player/StarModel/Star_AnimBP.OnPredationAttackStarted` _animbp (delegate `PredationAttackStart`))
      (add `/Game/Matsumoto/Player/StarModel/Star_AnimBP.OnPredationAttackEnded` _animbp (delegate `PredationAttackEnd`)))
    (:`then_1`
      (add `/Game/Matsumoto/Player/StarModel/Star_AnimBP.OnPredationEnd` (`/Game/Matsumoto/Player/BP_Player.AnimBP` Player) (delegate `PredationEnd`)))))

(event `PredationAttackStart`
  ;[1 1 1] Bind Collision
  (`/Game/Matsumoto/Player/BP_Player.SetCollision` (stale `self.Generated` Player) (stale `self.Generated` _primitivecomponent) true))

(event `PredationAttackEnd`
  ;[1 1 1] Bind Collision
  (`/Game/Matsumoto/Player/BP_Player.SetCollision` (stale `self.Generated` Player) (stale `self.Generated` _primitivecomponent) false))

(event `self.CollisionHitChild`
  (params (OverlappedComponent :type "PrimitiveComponent Object Reference") (OtherActor :type "Actor Object Reference") (OtherCompoent :type "PrimitiveComponent Object Reference") (OtherBodyIndex :type Integer) (FromSweep :type Boolean) (SweepResult :type "HitResult Structure"))
  (bind _basepower (`self.BasePower`))
  (bind _player (`self.Player`))
  (cast `/Game/Nakajima/AI/Enemy/StarEnemy/Pawn/EnemyCharacterBase` OtherActor
    (:`then`
      ;[1 1 1] Constant Add StarPower
      (`/Game/Matsumoto/Player/BP_Player.AddStarPower` _player 0.0625))
    (:`CastFailed`
      _))
  (`/Game/Matsumoto/Player/BP_Player.PlaySound` _player "/Game/Audio/eat-meat1.eat-meat1")
  (`GameplayStatics.ApplyDamage` OtherActor _basepower)
  (`KismetSystemLibrary.PrintString` null (`KismetStringLibrary.Concat_StrStr` "Hit Damage : " (`KismetStringLibrary.Conv_DoubleToString` _basepower))))

(event `PredationEnd`
  (`self.EndUse` (stale `self.Generated` Player)))

(fn `GetWeaponName`
  (returns (WeaponName :type Text))
  (return "Predation"))