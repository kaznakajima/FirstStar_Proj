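; BP_BossCore is a temporary, damageable core for a boss enemy that passes any damage it receives to its owner.
; On BeginPlay, a timeline animates its world Z into place, and after a fixed delay a second timeline, played in reverse, animates it out.
; When that finishes, the core calls SpawnClear on its owner and destroys itself.
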(event `self.ReceiveBeginPlay`
  (bind (_returnvalue_x _returnvalue_y) (`KismetMathLibrary.BreakVector` (`self.K2_GetActorLocation`)))
  (bind (_returnvalue_x_2 _returnvalue_y_2) (`KismetMathLibrary.BreakVector` (`self.K2_GetActorLocation`)))
  (bind (_direction _vector) (`Timeline|SpawnAnim` :!via `PlayFromStart`)
    (:`Update`
      (`self.K2_SetActorLocation` (`KismetMathLibrary.MakeVector` _returnvalue_x _returnvalue_y (.z _vector))))
    (:`Finished`
      (`KismetSystemLibrary.Delay` 15.0)
      (bind (_direction_2 _vector_2) (`Timeline|DestroyAnim` :!via `ReverseFromEnd`)
        (:`Update`
          (`self.K2_SetActorLocation` (`KismetMathLibrary.MakeVector` _returnvalue_x_2 _returnvalue_y_2 (.z _vector_2))))
        (:`Finished`
          (`/Game/Nakajima/AI/Enemy/BossEnemy/BP_BossCharacter.SpawnClear` (`self.MyOwner`))
          (`self.K2_DestroyActor`))))))

(event `self.ReceiveAnyDamage`
  (params (Damage :type "Float (single-precision)") (DamageType :type "DamageType Object Reference") (InstigatedBy :type "Controller Object Reference") (DamageCauser :type "Actor Object Reference"))
  (`GameplayStatics.ApplyDamage` (`self.MyOwner`) Damage))

(fn `UserConstructionScript`)