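; Boss enemy character that loads HP, attack power and move speed from DT_BossParamData and creates its UI_Boss widget.
; Short and long attacks toggle state flags around delays, with the long attack first turning toward the player.
; Arm overlaps damage the player, while ranged events reveal a held rock, then swap it for a spawned BP_Rock.
; Incoming damage drains HP through a timeline lerp and sets IsDeath at zero.
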(event `self.ReceiveBeginPlay`
  ;[1 1 1] ボスの初期化
  (bind (_hp _shortrangepower _longrangepower _movespeed) (`self.LoadParam`)) ; パラメータの取得
  (bind _output_get (set `self.MaxHP` _hp))
  (set `self.CurrentHP` _output_get)
  (set `self.ShortRangePower` _shortrangepower)
  (set `self.LongRangePower` _longrangepower)
  (set `self.MoveSpeed` _movespeed)
  (bind _returnvalue (`|CreateWidget` "/Game/Nakajima/Widget/UI_Boss.UI_Boss_C"))
  (set `/Game/Nakajima/Widget/UI_Boss.BossCharacter` self _returnvalue)
  (`UserWidget.AddToViewport` _returnvalue 0))

(event `/Game/Nakajima/AI/Enemy/StarEnemy/EnemyInterface.Attack`
  ;[1 1 1] 近距離攻撃
  (`self.AttackFunction` "AT_SHORTRANGE" (`self.FirstCombo`))
  (`KismetSystemLibrary.Delay` 0.5)
  (`self.AttackFunction` "AT_SHORTRANGE" (`self.FirstCombo`)))

(event `/Game/Nakajima/AI/Enemy/StarEnemy/EnemyInterface.LongAttack`
  ;[1 1 1] 遠距離攻撃
  (`self.LookPlayer`)
  (`self.AttackFunction` "AT_RONGRANGE" (`self.LongAttackFlg`))
  (`KismetSystemLibrary.Delay` 3.0)
  (`self.AttackFunction` "AT_RONGRANGE" (`self.LongAttackFlg`)))

(event `LookPlayer`
  (bind (_returnvalue_roll _returnvalue_pitch _returnvalue_yaw) (`KismetMathLibrary.BreakRotator` (`KismetMathLibrary.RInterpTo` (`self.K2_GetActorRotation`) (`KismetMathLibrary.FindLookAtRotation` (`self.K2_GetActorLocation`) (`self.K2_GetActorLocation` (`GameplayStatics.GetPlayerCharacter` 0))) (`GameplayStatics.GetWorldDeltaSeconds`))))
  ;[1 1 1] 遠距離攻撃
  (`self.K2_SetActorRotation` (`KismetMathLibrary.MakeRotator` 0.0 0.0 _returnvalue_yaw)))

(event `LongAttackStart`
  ;[1 1 1] 遠距離攻撃
  (`SceneComponent.SetHiddenInGame` (`self.Rock`) false false))

(event `SpawnRock`
  ;[1 1 1] 遠距離攻撃
  (bind _returnvalue (`|SpawnActorFromClass` "/Game/Nakajima/AI/Enemy/BossEnemy/BP_Rock.BP_Rock_C" (`SceneComponent.K2_GetComponentToWorld` (`self.SpawnPoint`)) "Undefined" "OverrideRootScale" null null))
  (set `/Game/Nakajima/AI/Enemy/BossEnemy/BP_Rock.MyOwner` self _returnvalue)
  (`SceneComponent.SetHiddenInGame` (`self.Rock`) true false))

(event `self.RightArm.OnComponentBeginOverlap`
  (params (OverlappedComponent :type "PrimitiveComponent Object Reference") (OtherActor :type "Actor Object Reference") (OtherComp :type "PrimitiveComponent Object Reference") (OtherBodyIndex :type Integer) (bFromSweep :type Boolean) (SweepResult :type "HitResult Structure (by ref)"))
  ;[1 1 1] 攻撃の当たり判定
  (bind _asthird_person_character (cast `/Game/ThirdPersonBP/Blueprints/ThirdPersonCharacter` OtherActor))
  (`GameplayStatics.ApplyDamage` _asthird_person_character (`self.ShortRangePower`))
  (`KismetSystemLibrary.PrintString` "Hit"))

(event `self.LeftArm.OnComponentBeginOverlap`
  (params (OverlappedComponent :type "PrimitiveComponent Object Reference") (OtherActor :type "Actor Object Reference") (OtherComp :type "PrimitiveComponent Object Reference") (OtherBodyIndex :type Integer) (bFromSweep :type Boolean) (SweepResult :type "HitResult Structure (by ref)"))
  ;[1 1 1] 攻撃の当たり判定
  (bind _asthird_person_character (cast `/Game/ThirdPersonBP/Blueprints/ThirdPersonCharacter` OtherActor))
  (`GameplayStatics.ApplyDamage` _asthird_person_character (`self.ShortRangePower`))
  (`KismetSystemLibrary.PrintString` "Hit"))

(event `self.ReceiveAnyDamage`
  (params (Damage :type "Float (single-precision)") (DamageType :type "DamageType Object Reference") (InstigatedBy :type "Controller Object Reference") (DamageCauser :type "Actor Object Reference"))
  ;[1 1 1] ダメージ処理
  (bind _output_get (set `self.TotalDamage` (`self.CurrentHP`)))
  (bind (_direction _deltatime) (`Timeline|Damage` :!via `PlayFromStart`)
    (:`Update`
      (bind _output_get_2 (set `self.CurrentHP` (`KismetMathLibrary.Lerp` _output_get (- (`self.TotalDamage`) Damage) _deltatime)))
      (if (<= _output_get_2 0.0)
        (set `self.IsDeath` true)))))

(fn `AttackFunction`
  (params (Type :type "EAttackType Enum" :default "AT_SHORTRANGE") (IsAttack :type Boolean))
  (bind _returnvalue (not IsAttack))
  (bind _output_get (set `self.AttackType` Type))
  (switch `EAttackType` _output_get
    (:`AT_SHORTRANGE`
      (set `self.FirstCombo` _returnvalue))
    (:`AT_RONGRANGE`
      (set `self.LongAttackFlg` _returnvalue))))

(fn `LoadParam`
  (returns (HP :type "Float (double-precision)") (ShortRangePower :type "Float (double-precision)") (LongRangePower :type "Float (double-precision)") (MoveSpeed :type "Float (double-precision)"))
  (bind _outrownames (`DataTableFunctionLibrary.GetDataTableRowNames` "/Game/Nakajima/AI/Enemy/BossEnemy/EnemyData/DT_BossParamData.DT_BossParamData"))
  (for _array_element _outrownames
    (bind _returnvalue (`|GetDataTableRow` "/Game/Nakajima/AI/Enemy/BossEnemy/EnemyData/DT_BossParamData.DT_BossParamData" _array_element)
      (:`then`
        (bind (_hp _shortrangepower _longrangepower _movespeed) (break `/Game/Nakajima/AI/Enemy/BossEnemy/EnemyData/S_BossParam` _returnvalue))
        (return _hp _shortrangepower _longrangepower _movespeed)))))

(fn `UserConstructionScript`)