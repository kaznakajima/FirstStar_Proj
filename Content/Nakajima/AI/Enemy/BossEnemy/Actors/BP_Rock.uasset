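; BP_Rock is a breakable rock in the boss enemy's actors that damages the player using its owner's LongRangePower.
; It enables physics simulation on the Rock component shortly after BeginPlay and applies damage only on the first hit against BP_Player.
; When the component fractures, it stops colliding with pawns and destroys itself after a short delay.
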(event `self.ReceiveBeginPlay`
  (`KismetSystemLibrary.Delay` 0.5)
  (`PrimitiveComponent.SetSimulatePhysics` (`self.Rock`) true))

(event `self.Rock.OnComponentHit`
  (params (HitComponent :type "PrimitiveComponent Object Reference") (OtherActor :type "Actor Object Reference") (OtherComp :type "PrimitiveComponent Object Reference") (NormalImpulse :type "Vector Structure") (Hit :type "HitResult Structure (by ref)"))
  (bind _asbp_player (cast `/Game/Matsumoto/Player/BP_Player` OtherActor))
  (`/Engine/EditorBlueprintResources/StandardMacros.DoOnce` false
    (:`Completed`
      (`GameplayStatics.ApplyDamage` _asbp_player (`BossCharacter.LongRangePower` (`self.MyOwner`))))))

(event `self.Rock.OnComponentFracture`
  (params (HitPoint :type "Vector Structure (by ref)") (HitDirection :type "Vector Structure (by ref)"))
  (`/Engine/EditorBlueprintResources/StandardMacros.DoOnce` false
    (:`Completed`
      (`PrimitiveComponent.SetCollisionResponseToChannel` (`self.Rock`) "ECC_Pawn" "ECR_Ignore")
      (`KismetSystemLibrary.Delay` 2.0)
      (`self.K2_DestroyActor`))))

(fn `UserConstructionScript`)