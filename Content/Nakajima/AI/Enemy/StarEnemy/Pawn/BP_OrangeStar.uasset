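; BP_OrangeStar is the orange variant of the star enemy pawn, a child Blueprint that can explode.
; On BeginPlay it tags its type as ORANGE, runs the parent setup, then applies Speed to its floating movement and prints the result.
; Its Explosion event spawns a BP_Explosion at its transform, passes on its Power and destroys the star.
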(event `self.ReceiveBeginPlay`
  (set `self.Type` "ET_ORANGE")
  (`parent.ReceiveBeginPlay`)
  (bind _output_get (set `FloatingPawnMovement.MaxSpeed` (`self.Speed`) (`self.GetFloatingMovement`)))
  (`KismetSystemLibrary.PrintString` (`KismetStringLibrary.Conv_DoubleToString` _output_get)))

(event `/Game/Nakajima/AI/Enemy/StarEnemy/EnemyInterface.Explosion`
  (bind _returnvalue (`|SpawnActorFromClass` "/Game/Nakajima/AI/Enemy/StarEnemy/BP_Explosion.BP_Explosion_C" (`self.GetTransform`) "Undefined" "OverrideRootScale" null null))
  (set `/Game/Nakajima/AI/Enemy/StarEnemy/BP_Explosion.Power` (`self.Power`) _returnvalue)
  (`self.K2_DestroyActor`))

(fn `UserConstructionScript`
  (`parent.UserConstructionScript`))