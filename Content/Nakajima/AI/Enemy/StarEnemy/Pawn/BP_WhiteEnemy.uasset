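; BP_WhiteEnemy is a flying enemy that always faces the player and fires ranged attacks.
; BeginPlay loads HP, speed and power by Type, applies the fly speed and sets up an HP UI that Tick repositions.
; Attack spawns BP_Attack at the enemy's transform.
; Damage spawns a hit effect and drains HP through a timeline lerp, flagging death and ignoring Pawn collision at zero.
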(event `self.ReceiveBeginPlay`
  ;[1 1 1] 初期化
  (bind (_hp _groundsp _fluingsp _s_power _l_power) (`self.LoadParam` (`self.Type`)))
  (bind _output_get (set `self.MaxHP` _hp))
  (set `self.CurrentHP` _output_get)
  (bind _output_get_2 (set `self.MoveSpeed` _groundsp))
  (set `self.ShortRangePower` _s_power)
  (set `self.LongRangePower` _l_power)
  (set `CharacterMovementComponent.MaxFlySpeed` _output_get_2 (`self.CharacterMovement`))
  (`self.SetUI`))

(event `/Game/Nakajima/AI/Enemy/EnemyInterface.Attack`
  ;[1 1 1] 遠距離攻撃
  (`|SpawnActorFromClass` "/Game/Nakajima/AI/Enemy/StarEnemy/Actors/BP_Attack.BP_Attack_C" (`self.GetTransform`) "Undefined" "OverrideRootScale" null null))

(event `self.ReceiveAnyDamage`
  (params (Damage :type "Float (single-precision)") (DamageType :type "DamageType Object Reference") (InstigatedBy :type "Controller Object Reference") (DamageCauser :type "Actor Object Reference"))
  (`|SpawnActorFromClass` "/Game/Nakajima/AI/Enemy/StarEnemy/Actors/BP_HitEffect.BP_HitEffect_C" (`self.GetTransform`) "Undefined" "OverrideRootScale" null null)
  (bind _output_get (set `self.TotalDamage` (`self.CurrentHP`)))
  (bind (_direction _deltatime) (`Timeline|Damage` :!via `PlayFromStart`)
    (:`Update`
      (bind _output_get_2 (set `self.CurrentHP` (`KismetMathLibrary.Lerp` _output_get (- (`self.TotalDamage`) Damage) _deltatime)))
      (if (<= _output_get_2 0.0)
        (set `self.IsDeath` true)
        (`self.IgnoreCollision`)))))

(event `self.ReceiveTick`
  (params (DeltaSeconds :type "Float (single-precision)"))
  (bind _myhp_ui (`self.MyHP_UI`))
  ;[1 1 1] 常にプレイヤー方向を向く
  (`self.K2_SetActorRotation` (`KismetMathLibrary.FindLookAtRotation` (`self.K2_GetActorLocation`) (`self.K2_GetActorLocation` (`GameplayStatics.GetPlayerCharacter` 0))))
  (if (`KismetSystemLibrary.IsValid` _myhp_ui)
    (`/Game/Nakajima/Widget/UI_StarEnemy.SetUIPosition` _myhp_ui)))

(event `self.IgnoreCollision`
  (`PrimitiveComponent.SetCollisionResponseToChannel` (`self.Collision`) "ECC_Pawn" "ECR_Ignore")
  (`PrimitiveComponent.SetCollisionResponseToChannel` (`self.CapsuleComponent`) "ECC_Pawn" "ECR_Ignore"))

(fn `UserConstructionScript`
  (`parent.UserConstructionScript`))