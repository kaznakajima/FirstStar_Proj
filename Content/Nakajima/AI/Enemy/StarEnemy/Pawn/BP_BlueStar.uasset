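; BP_BlueStar is the blue variant of the star enemy pawn, with a ranged attack and a self-destruct attack.
; BeginPlay sets its type to BLUE, runs the parent setup, then applies Speed to the floating movement and prints it.
; Attack spawns BP_Attack at the pawn's transform, gated by a Delay-based cooldown flag.
; Explosion spawns BP_Explosion, passes it Power, and destroys the pawn.
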(event `self.ReceiveBeginPlay`
  ;[1 1 1] 初期化
  (set `self.Type` "ET_BLUE")
  (`parent.ReceiveBeginPlay`)
  (bind _output_get (set `FloatingPawnMovement.MaxSpeed` (`self.Speed`) (`self.GetFloatingMovement`)))
  (`KismetSystemLibrary.PrintString` (`KismetStringLibrary.Conv_DoubleToString` _output_get)))

(event `/Game/Nakajima/AI/Enemy/StarEnemy/EnemyInterface.Explosion`
  ;[1 1 1] 自爆攻撃
  (bind _returnvalue (`|SpawnActorFromClass` "/Game/Nakajima/AI/Enemy/StarEnemy/Actors/BP_Explosion.BP_Explosion_C" (`self.GetTransform`) "Undefined" "OverrideRootScale" null null))
  (set `/Game/Nakajima/AI/Enemy/StarEnemy/Actors/BP_Explosion.Power` (`self.Power`) _returnvalue)
  (`self.K2_DestroyActor`))

(event `/Game/Nakajima/AI/Enemy/StarEnemy/EnemyInterface.Attack`
  ;[1 1 1] 遠距離攻撃
  (if (not (`self.IsAttack`))
    (`|SpawnActorFromClass` "/Game/Nakajima/AI/Enemy/StarEnemy/Actors/BP_Attack.BP_Attack_C" (`self.GetTransform`) "Undefined" "OverrideRootScale" null null)
    (set `self.IsAttack` true)
    (`KismetSystemLibrary.Delay` 2.0)
    (set `self.IsAttack` false)))

(fn `UserConstructionScript`
  (`parent.UserConstructionScript`))