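; BP_EnemyBase is an enemy base Blueprint that configures itself from the DT_EnemyData table according to its EnemyType.
; LoadData converts the type to an integer index into the table's row names, so row order must match the type values.
; It returns the row's stats, class, behaviour and material.
; BeginPlay applies only HP, attack power and the mesh material; Tick and overlap events are unused.
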(event `self.ReceiveBeginPlay`
  (bind (_myclass _hp _groundsp _flyingsp _attackpower _mybehaviour _material) (`self.LoadData` (`self.EnemyType`)))
  (set `self.HP` _hp)
  (set `self.Power` _attackpower)
  (`PrimitiveComponent.SetMaterial` (`self.MeshComponent`) 0 _material))

(fn `LoadData`
  (params (Type :type "/Game/Nakajima/AI/Enemy/EnemyData/EnemyType Enum" :default "NewEnumerator4"))
  (returns (MyClass :type "Pawn Class Reference") (HP :type "Float (double-precision)") (GroundSp :type "Float (double-precision)") (FlyingSp :type "Float (double-precision)") (AttackPower :type "Float (double-precision)") (MyBehaviour :type "BehaviorTree Object Reference") (Material :type "Material Object Reference"))
  ;[1 1 1] データテーブルからパラメータ取得
  (bind _outrownames (`DataTableFunctionLibrary.GetDataTableRowNames` "/Game/Nakajima/AI/Enemy/EnemyData/DT_EnemyData.DT_EnemyData"))
  (bind _returnvalue (`|GetDataTableRow` "/Game/Nakajima/AI/Enemy/EnemyData/DT_EnemyData.DT_EnemyData" (`|GetArrayItem` _outrownames (`KismetMathLibrary.Conv_ByteToInt` Type)))
    (:`then`
      (bind (_myclass _hp _groundsp _flyingsp _attackpower _mybehaviour _enemymaterial) (break `/Game/Nakajima/AI/Enemy/EnemyData/S_EnemyParam` _returnvalue))
      (return _myclass _hp _groundsp _flyingsp _attackpower _mybehaviour _enemymaterial) ; 該当する敵タイプのパラメータを返す
    )))

(fn `UserConstructionScript`)