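; Orange star-enemy pawn that flies, always faces the player and has ranged and arm attacks.
; BeginPlay loads HP, speed and power by type and creates the HP UI, which follows it each tick.
; Attack spawns BP_Attack, while SetCollision toggles arm hitboxes; left-arm overlaps pass a DoOnce to damage the player using long-range power.
; Incoming damage drains HP through a timeline, destroying enemy and UI at zero.
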(event `self.ReceiveBeginPlay`
  ;[1 1 1] 初期化
  (bind (_hp _groundsp _fluingsp _s_power _l_power) (`self.LoadParam` (`self.Type`)))
  (bind _output_get (set `self.MaxHP` _hp))
  (set `self.CurrentHP` _output_get)
  (bind _output_get_2 (set `self.MoveSpeed` _groundsp))
  (set `self.ShortRangePower` _s_power)
  (set `self.LongRangePower` _l_power)
  (set `CharacterMovementComponent.MaxFlySpeed` _output_get_2 (`self.CharacterMovement`))
  (`self.SetUI`)
  (`self.SetCollision` false "Right")
  (`self.SetCollision` false "Left"))

(event `/Game/Nakajima/AI/Enemy/StarEnemy/EnemyInterface.Attack`
  ;[1 1 1] 遠距離攻撃
  (`|SpawnActorFromClass` "/Game/Nakajima/AI/Enemy/StarEnemy/BP_Attack.BP_Attack_C" (`self.GetTransform`) "Undefined" "OverrideRootScale" null null))

(event `self.ReceiveTick`
  (params (DeltaSeconds :type "Float (single-precision)"))
  (bind _myhp_ui (`self.MyHP_UI`))
  ;[1 1 1] 常にプレイヤー方向を向く
  (`self.K2_SetActorRotation` (`KismetMathLibrary.FindLookAtRotation` (`self.K2_GetActorLocation`) (`self.K2_GetActorLocation` (`GameplayStatics.GetPlayerCharacter` 0))))
  (if (`KismetSystemLibrary.IsValid` _myhp_ui)
    (`/Game/Nakajima/Widget/UI_StarEnemy.SetUIPosition` _myhp_ui)))

(event `self.SetCollision`
  (params (Isactive :type Boolean) (ArmName :type Name))
  (bind _righttapcol (`self.RightTapCol`))
  (bind _lefttapcol (`self.LeftTapCol`))
  ;[1 1 1] 当たり判定のアクティブ化
  (switch `name` ArmName
    (:`Right`
      (if Isactive
        (`PrimitiveComponent.SetCollisionEnabled` _righttapcol "QueryAndPhysics")
        (else
          (`PrimitiveComponent.SetCollisionEnabled` _righttapcol "NoCollision")
          (goto _label :!via `Reset`))))
    (:`Left`
      (if Isactive
        (`PrimitiveComponent.SetCollisionEnabled` _lefttapcol "QueryAndPhysics")
        (else
          (`PrimitiveComponent.SetCollisionEnabled` _lefttapcol "NoCollision")
          (goto _label :!via `Reset`))))))

(event `self.LeftTapCol.OnComponentBeginOverlap`
  (params (OverlappedComponent :type "PrimitiveComponent Object Reference") (OtherActor :type "Actor Object Reference") (OtherComp :type "PrimitiveComponent Object Reference") (OtherBodyIndex :type Integer) (bFromSweep :type Boolean) (SweepResult :type "HitResult Structure (by ref)"))
  ;[1 1 1] 当たり判定のアクティブ化
  (bind _asbp_player (cast `/Game/Matsumoto/Player/BP_Player` OtherActor))
  (`/Engine/EditorBlueprintResources/StandardMacros.DoOnce` false :!label _label
    (:`Completed`
      (`GameplayStatics.ApplyDamage` _asbp_player (`self.LongRangePower`)))))

(event `self.ReceiveAnyDamage`
  (params (Damage :type "Float (single-precision)") (DamageType :type "DamageType Object Reference") (InstigatedBy :type "Controller Object Reference") (DamageCauser :type "Actor Object Reference"))
  (bind _output_get (set `self.TotalDamage` (`self.CurrentHP`)))
  (bind (_direction _deltatime) (`Timeline|Damage` :!via `PlayFromStart`)
    (:`Update`
      (bind _output_get_2 (set `self.CurrentHP` (`KismetMathLibrary.Lerp` _output_get (- (`self.TotalDamage`) Damage) _deltatime)))
      (if (<= _output_get_2 0.0)
        (`self.DeleteUI`)
        (`self.K2_DestroyActor`)))))

(fn `UserConstructionScript`
  (`parent.UserConstructionScript`))