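; White star enemy character that spawns as a randomly chosen enemy type.
; On BeginPlay it rolls one of five types and looks up that type's stats in DT_EnemyData, matching the enum value to the row's index.
; It applies the row's material to the mesh and uses GroundSp, not FlyingSp, as max fly speed.
; HP and attack power are returned by the lookup but not applied here.
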(event `self.ReceiveBeginPlay`
  (bind _output_get (set `self.EnemyType` (cast `/Game/Nakajima/AI/Enemy/EnemyData/EnemyType` (`KismetMathLibrary.Conv_IntToByte` (`KismetMathLibrary.RandomInteger` 5)))))
  (bind (_hp _groundsp _flyingsp _attackpower _enemymaterial) (`self.LoadEnemyData` _output_get))
  (set `CharacterMovementComponent.MaxFlySpeed` _groundsp (`self.CharacterMovement`))
  (`PrimitiveComponent.SetMaterial` (`self.Mesh`) 0 _enemymaterial))

(fn `LoadEnemyData`
  (params (Type :type "/Game/Nakajima/AI/Enemy/EnemyData/EnemyType Enum" :default "NewEnumerator4"))
  (returns (HP :type Integer) (GroundSp :type "Float (double-precision)") (FlyingSp :type "Float (double-precision)") (AttackPower :type Integer) (Enemymaterial :type "Material Object Reference"))
  ;[1 1 1] データテーブルからパラメータ取得
  (bind _outrownames (`DataTableFunctionLibrary.GetDataTableRowNames` "/Game/Nakajima/AI/Enemy/EnemyData/DT_EnemyData.DT_EnemyData"))
  (for (_array_element _array_index) _outrownames
    (if (== _array_index (`KismetMathLibrary.Conv_ByteToInt` Type))
      (bind _returnvalue (`|GetDataTableRow` "/Game/Nakajima/AI/Enemy/EnemyData/DT_EnemyData.DT_EnemyData" _array_element)
        (:`then`
          (bind (_hp _groundsp _flyingsp _attackpower _attackrange _enemymaterial) (break `/Game/Nakajima/AI/Enemy/EnemyData/S_EnemyParam` _returnvalue))
          (return _hp _groundsp _flyingsp _attackpower _enemymaterial) ; 該当する敵タイプのパラメータを返す
        ))))
  (return 0 0.0 0.0 0 null) ; 見つからない場合は初期値を返す
)

(fn `UserConstructionScript`)