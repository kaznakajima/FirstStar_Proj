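; BP_Explosion is the Star Enemy's explosion actor, damaging the player caught in its expanding blast.
; On BeginPlay it reads ShortRangePower from its owning EnemyCharacterBase, then plays a timeline that grows the Sphere collision radius.
; Players overlapping the sphere take that power as damage, and the actor destroys itself when the Explosion effect system finishes.
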(event `self.ReceiveBeginPlay`
  (bind _asenemy_character_base (cast `/Game/Nakajima/AI/Enemy/StarEnemy/Pawn/EnemyCharacterBase` (`self.GetOwner`)))
  (set `self.Power` (`EnemyCharacter.ShortRangePower` _asenemy_character_base))
  (bind (_direction _size) (`Timeline|Collision` :!via `PlayFromStart`)
    (:`Update`
      (`SphereComponent.SetSphereRadius` (`self.Sphere`) (* _size 100.0) true))))

(event `self.Sphere.OnComponentBeginOverlap`
  (params (OverlappedComponent :type "PrimitiveComponent Object Reference") (OtherActor :type "Actor Object Reference") (OtherComp :type "PrimitiveComponent Object Reference") (OtherBodyIndex :type Integer) (bFromSweep :type Boolean) (SweepResult :type "HitResult Structure (by ref)"))
  (bind _asbp_player (cast `/Game/Matsumoto/Player/BP_Player` OtherActor))
  (`GameplayStatics.ApplyDamage` _asbp_player (`self.Power`)))

(event `self.Explosion.OnSystemFinished`
  (params (PSystem :type "ParticleSystemComponent Object Reference"))
  (`self.K2_DestroyActor`))

(fn `UserConstructionScript`)