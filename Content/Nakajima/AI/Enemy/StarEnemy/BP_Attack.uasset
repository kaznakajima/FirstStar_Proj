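; BP_Attack is a projectile actor for the Star enemy's attack, launched toward the player.
; On BeginPlay it rotates to face the first player character and sets its ProjectileMovement velocity along the vector to that position.
; The direction is not normalized, so speed scales with the distance to the player at spawn.
; The graph aims only once and holds no overlap, damage or tick logic.
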(event `self.ReceiveBeginPlay`
  (`self.K2_SetActorRotation` (`KismetMathLibrary.FindLookAtRotation` (`self.K2_GetActorLocation`) (`self.K2_GetActorLocation` (`GameplayStatics.GetPlayerCharacter` 0))))
  (set `MovementComponent.Velocity` (* (- (`self.K2_GetActorLocation` (`GameplayStatics.GetPlayerCharacter` 0)) (`self.K2_GetActorLocation`)) 5.0) (`self.ProjectileMovement`)))

(fn `UserConstructionScript`)