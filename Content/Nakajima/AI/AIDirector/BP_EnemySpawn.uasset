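; Enemy spawn point in the AI Director folder that spawns an AI pawn at its own location on BeginPlay.
; GetEnemyParam resolves its Type to the pawn class and behavior tree to spawn, using a fixed rotation.
; A separate SpawnEnemy event, not called here, loops over DT_EnemyData rows, spawning those whose index matches a random roll in the loop.
; Its switch takes a constant, and all cases share one spawn path.
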(event `self.ReceiveBeginPlay`
  (bind _param (`self.GetEnemyParam` (`self.Type`)))
  (bind (_myclass _hp _groundsp _flyingsp _s_power _l_power _mybehaviour) (break `/Game/Nakajima/AI/Enemy/StarEnemy/EnemyData/S_EnemyParam` _param))
  (`AIBlueprintHelperLibrary.SpawnAIFromClass` _myclass _mybehaviour (`self.K2_GetActorLocation`) (struct :`Yaw` 90.0)))

(event `SpawnEnemy`
  (bind _outrownames (`DataTableFunctionLibrary.GetDataTableRowNames` "/Game/Nakajima/AI/Enemy/StarEnemy/EnemyData/DT_EnemyData.DT_EnemyData"))
  (for (_array_element _array_index) _outrownames
    (if (== _array_index (`KismetMathLibrary.RandomInteger` 5))
      (switch `int` 2
        (:`0`
          _)
        (:`1`
          _)
        (:`2`
          _)
        (:`3`
          _)
        (:`4`
          _))
      (bind _returnvalue (`|GetDataTableRow` "/Game/Nakajima/AI/Enemy/StarEnemy/EnemyData/DT_EnemyData.DT_EnemyData" _array_element)
        (:`then`
          (bind (_myclass _hp _groundsp _flyingsp _s_power _l_power _mybehaviour) (break `/Game/Nakajima/AI/Enemy/StarEnemy/EnemyData/S_EnemyParam` _returnvalue))
          (`AIBlueprintHelperLibrary.SpawnAIFromClass` _myclass _mybehaviour (`self.K2_GetActorLocation`)))))))

(fn `UserConstructionScript`
  (`parent.UserConstructionScript`))